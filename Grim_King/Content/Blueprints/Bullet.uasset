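; Bullet actor that damages the third-person player character when its sphere collision begins an overlap, apparently as a boss projectile.
; A hit subtracts a fixed amount of Health unless the character is Blocking, then prints the new value.
; The bullet ignores Boss_Enemy and destroys itself on any other non-player actor.
; It is not destroyed on overlapping the player, whether blocked or not.
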(event `self.Sphere1.OnComponentBeginOverlap`
  (params (OverlappedComponent :type "PrimitiveComponent Object Reference") (OtherActor :type "Actor Object Reference") (OtherComp :type "PrimitiveComponent Object Reference") (OtherBodyIndex :type Integer) (bFromSweep :type Boolean) (SweepResult :type "HitResult Structure (by ref)"))
  (bind _asbp_third_person_character (cast `/Game/ThirdPerson/Blueprints/BP_ThirdPersonCharacter` OtherActor)
    (:`then`
      (if (not (`/Game/ThirdPerson/Blueprints/BP_ThirdPersonCharacter.blocking` _asbp_third_person_character))
        (bind _output_get (set `/Game/ThirdPerson/Blueprints/BP_ThirdPersonCharacter.health` (- (`/Game/ThirdPerson/Blueprints/BP_ThirdPersonCharacter.health` _asbp_third_person_character) 5) _asbp_third_person_character))
        (`KismetSystemLibrary.PrintString` (`KismetStringLibrary.Conv_IntToString` _output_get))))
    (:`CastFailed`
      (cast `/Game/Blueprints/Boss_Enemy` OtherActor
        (:`CastFailed`
          (`KismetSystemLibrary.PrintString` "Not boss")
          (`self.K2_DestroyActor`))))))

(fn `UserConstructionScript`)